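; PickupManager randomly populates a deployed actor's socket locations with obstacles and gold rewards.
; DeployPickups waits briefly, then collects PickupSocket locations from the instigator's visible static mesh child components.
; RandomizePickups rolls per location to add one of two obstacle types (commented fire or lantern) as child actor components of the manager.
; A further roll, only where an obstacle spawns, adds gold at that same spot.
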(event Custom|DeployPickups
  (params (Instigator :type Actor%20Object%20Reference))
  (bind _potentiallocations (Variables|Default|GetPotentialLocations))
  (Utilities|FlowControl|Delay 0.2)
  (for _array_element (Components|GetChildrenComponents (VehicleSound|GetRootComponent Instigator) true)
    (bind _asstatic_mesh_component (Utilities|Casting|CastToStaticMeshComponent _array_element))
    (if (Rendering|IsVisible _asstatic_mesh_component)
      (if (Transformation|DoesSocketExist _asstatic_mesh_component "PickupSocket")
        (Utilities|Array|Add (Variables|Default|GetPotentialLocations) (Transformation|GetSocketLocation _asstatic_mesh_component "PickupSocket")))))
  (CallFunction|RandomizePickups _potentiallocations)
  (Utilities|Array|Clear _potentiallocations))

(fn ConstructionScript)

(fn RandomizePickups
  (params (Locations :type Array%20of%20Vectors))
  (for _array_element Locations
    ;[1 1 1] To Spawn or Not to Spawn
    (if (> (Math|Random|RandomFloatinRange 0.0 1.0) 0.8)
      ;[1 1 1] Select Obstacle to Spawn
      (if (> (Math|Random|RandomFloatinRange 0.0 1.0) 0.5)
        ;[1 1 1] Fire or Lantern
        (AddComponent|AddChildActorComponent false (Math|Transform|MakeTransform (- _array_element (Transformation|GetActorLocation))))
        (else
          (AddComponent|AddChildActorComponent false (Math|Transform|MakeTransform (- _array_element (Transformation|GetActorLocation))))))
      ;[1 1 1] Should Spawn Reward?
      (if (> (Math|Random|RandomFloatinRange 0.0 1.0) 0.8)
        ;[1 1 1] Spawn Gold
        (AddComponent|AddChildActorComponent false (Math|Transform|MakeTransform (- _array_element (Transformation|GetActorLocation))))))))