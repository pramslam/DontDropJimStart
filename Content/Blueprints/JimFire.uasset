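; JimFire is a fire hazard that kills Jim on contact and can be removed by repeated clicks.
; On overlap it freezes player and level-item movement through JimGame, plays the death sound and animation, then destroys the character and calls JimDies after a short delay.
; While player movement is allowed, each mouse release advances a click counter until the fire awards score, plays a pickup sound and destroys itself.
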(event EventBeginPlay
  ;[1 1 1] Setup Game Class
  (bind _asjim_game (Utilities|Casting|CastToJimGame (Game|GetGameMode)))
  (Variables|Default|SetJimGame _asjim_game))

(event Collision|EventActorBeginOverlap
  (params (OtherActor :type Actor%20Object%20Reference))
  (bind _jimgame (Variables|Default|GetJimGame))
  ;[1 1 1] Setup Character Class
  (bind _asjim_character (Utilities|Casting|CastToJimCharacter OtherActor))
  (Variables|Default|SetJimCharacter _asjim_character)
  ;[1 1 1] Play Animation and Sound  on Death
  (Variables|Default|Setactive false)
  (Variables|/Game/Blueprints/JimGame.JimGame_C|SetCanMoveLevelItems _jimgame false)
  (Variables|/Game/Blueprints/JimGame.JimGame_C|SetCanMovePlayer _jimgame false)
  (Audio|Components|Audio|Play (Variables|/Game/Blueprints/JimGame.JimGame_C|GetDeathSound (Variables|Default|GetJimGame)) 0.0)
  (bind _asbp_jim_anims (Utilities|Casting|CastToBP_Jim_Anims (Components|SkeletalMesh|GetAnimInstance (Variables|/Script/Engine.Character|GetMesh (Variables|Default|GetJimCharacter)))))
  (Variables|Default|SetJimAnims _asbp_jim_anims)
  (Variables|/Game/JimCharacter/BP_Jim_Anims.BP_Jim_Anims_C|SetIsNotDead? (Variables|Default|GetJimAnims) false)
  (Variables|/Game/JimCharacter/BP_Jim_Anims.BP_Jim_Anims_C|SetIsDead (Variables|Default|GetJimAnims) true)
  (Utilities|FlowControl|Delay 0.8)
  (Actor|DestroyActor (Variables|Default|GetJimCharacter))
  (Default|JimDies (Variables|Default|GetJimGame)))

(event EventActorOnReleased
  ;[1 1 1] Fire Touched
  (if (Variables|/Game/Blueprints/JimGame.JimGame_C|GetCanMovePlayer (Variables|Default|GetJimGame))
    (Utilities|FlowControl|Delay 0.03)
    (if (== (Variables|Default|GetClickedOn) 2)
      (Variables|/Game/Blueprints/JimGame.JimGame_C|SetScore (Variables|Default|GetJimGame) (+ 200 (Variables|/Game/Blueprints/JimGame.JimGame_C|GetScore (Variables|Default|GetJimGame))))
      (Audio|Components|Audio|Play (Variables|/Game/Blueprints/JimGame.JimGame_C|GetPickupSuccess (Variables|Default|GetJimGame)) 0.0)
      (Actor|DestroyActor)
      (else
        (Variables|Default|SetClickedOn (+ (Variables|Default|GetClickedOn) 1))))))

(fn ConstructionScript)