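; HUD for the Jim game that draws the title menu, in-game score and game over screen on the canvas.
; DrawHUD picks the screen from two menu flags, cutting buttons and panels from one UI texture atlas by UV and offsetting them from screen center.
; Hitboxes make Play and Reset clickable, calling the JimGame game mode cached at BeginPlay to enable movement and start, or reset after a short delay.
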(event Custom|DrawScore
  ;[1 1 1] Draw Score
  (if (not (Variables|Default|GetDrawGameOverMenu))
    (HUD|DrawText "SCORE: " "(R=1.000000,G=1.000000,B=1.000000,A=1.000000)" (- (* (Variables|Default|GetResX) 0.5) 75.0) 0.25 "/Game/DontDropJimAssets/JimFont.JimFont" 1.0 false)
    (HUD|DrawText (Utilities|String|ToString(Integer) (Variables|Default|GetCurrentScore)) "(R=1.000000,G=1.000000,B=1.000000,A=1.000000)" (- (* (Variables|Default|GetResX) 0.5) -75.0) 0.25 "/Game/DontDropJimAssets/JimFont.JimFont" 1.0 false)))

(event EventBeginPlay
  ;[1 1 1] Set the Game Store
  (bind _asjim_game (Utilities|Casting|CastToJimGame (Game|GetGameMode)))
  (Variables|Default|SetJimGameStore _asjim_game))

(event EventDrawHUD
  (params (SizeX :type Integer) (SizeY :type Integer))
  ;[1 1 1] Get Screen Resolution
  (Variables|Default|SetResX SizeX)
  (Variables|Default|SetResY SizeY)
  (if (Variables|Default|GetDrawGameOverMenu)
    ;[1 1 1] Draw Reset Button
    (Canvas|DrawTexture (Variables|Default|GetUITexture) (- (* (Variables|Default|GetResX) 0.5) (* (Variables|Default|GetResetXPos) 0.5)) (Variables|Default|GetResetYPos) (Variables|Default|GetResetXSize) (Variables|Default|GetResetYSize) 0.604 0.012 0.19 0.197 "(R=1.000000,G=1.000000,B=1.000000,A=1.000000)" "BLEND_Masked")
    ;[1 1 1] Hitbox for Reset Button
    (Class|HUD|AddHitBox (Math|Vector2D|MakeVector2D (- (* (Variables|Default|GetResX) 0.5) (* (Variables|Default|GetResetXPos) 0.5)) (Variables|Default|GetResetYPos)) (Math|Vector2D|MakeVector2D (Variables|Default|GetResetXSize) (Variables|Default|GetResetYSize)) (Variables|Default|GetResetHitbox) false)
    ;[1 1 1] Draw Score Menu
    (Canvas|DrawTexture (Variables|Default|GetUITexture) (- (* (Variables|Default|GetResX) 0.5) (* (Variables|Default|GetScoreXPos) 0.5)) (Variables|Default|GetScoreYPos) (Variables|Default|GetScoreXSize) (Variables|Default|GetScoreYSize) 0.222 0.389 0.565 0.23 "(R=1.000000,G=1.000000,B=1.000000,A=1.000000)" "BLEND_Masked")
    (elif (Variables|Default|GetDrawGameMenu)
      ;[1 1 1] Draw Play Button
      (Canvas|DrawTexture (Variables|Default|GetUITexture) (- (* (Variables|Default|GetResX) 0.5) (* (Variables|Default|GetPlayXPos) 0.5)) (Variables|Default|GetPlayYPos) (Variables|Default|GetPlayXSize) (Variables|Default|GetPlayYSize) 0.0147 0.238 0.2 0.197 "(R=1.000000,G=1.000000,B=1.000000,A=1.000000)" "BLEND_Masked")
      ;[1 1 1] Hitbox for Play Button
      (Class|HUD|AddHitBox (Math|Vector2D|MakeVector2D (- (* (Variables|Default|GetResX) 0.5) (* (Variables|Default|GetPlayXPos) 0.5)) (Variables|Default|GetPlayYPos)) (Math|Vector2D|MakeVector2D (Variables|Default|GetPlayXSize) (Variables|Default|GetPlayYSize)) (Variables|Default|GetPlayHitbox) false)
      ;[1 1 1] Draw Title Menu
      (Canvas|DrawTexture (Variables|Default|GetUITexture) (- (* (Variables|Default|GetResX) 0.5) (* (Variables|Default|GetLogoXPos) 0.5)) (Variables|Default|GetLogoYPos) (Variables|Default|GetLogoXSize) (Variables|Default|GetLogoYSize) 0.006 0.003 0.572 0.226 "(R=1.000000,G=1.000000,B=1.000000,A=1.000000)" "BLEND_Masked")
      (else
        (CallFunction|DrawScore)))))

(event EventHitBoxClick
  (params (BoxName :type Name))
  ;[1 1 1] If Clicked on a Hitbox
  (if (Utilities|Name|Equal(Name) BoxName (Variables|Default|GetPlayHitbox))
    (Variables|Default|SetDrawGameMenu false)
    (Audio|Components|Audio|Play (Variables|Default|GetButtonClick) 0.0)
    (Variables|/Game/Blueprints/JimGame.JimGame_C|SetCanMoveLevelItems (Variables|Default|GetJimGameStore) true)
    (Variables|/Game/Blueprints/JimGame.JimGame_C|SetCanMovePlayer (Variables|Default|GetJimGameStore) true)
    (Default|StartGame (Variables|Default|GetJimGameStore))
    (elif (Utilities|Name|Equal(Name) BoxName (Variables|Default|GetResetHitbox))
      (Audio|Components|Audio|Play (Variables|Default|GetButtonClick) 0.0)
      (Utilities|FlowControl|Delay 0.1)
      (Default|ResetGame (Variables|Default|GetJimGameStore)))))

(fn ConstructionScript)