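; UpperPlatformSet is one of two swapping platform sets, randomly building a six-row grid of visible, collidable platforms and gaps when CreateSelf fires.
; BeginPlay caches TopPlatformSet and the other UpperPlatformSet instance.
; CreateSelf seeds row one from TopPlatformSet's Gaps, then GeneratePlatforms chains rows two to six.
; Each row places platforms over the previous row's gaps, matched by numeric component names, then randomly fills up to five, recording new gaps.
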(event Custom|CreateSelf
  (bind _1_1 (Variables|PlatformMeshes|Get1.1))
  (bind _1_2 (Variables|PlatformMeshes|Get1.2))
  (bind _1_3 (Variables|PlatformMeshes|Get1.3))
  (bind _1_4 (Variables|PlatformMeshes|Get1.4))
  (bind _1_5 (Variables|PlatformMeshes|Get1.5))
  (bind _1_6 (Variables|PlatformMeshes|Get1.6))
  (bind _array (Utilities|Array|MakeArray _1_1 _1_2 _1_3 _1_4 _1_5 _1_6))
  ;[1 1 1] Create Self Sequence
  (Utilities|FlowControl|Sequence
    (:then_0
      ;[1 1 1] Setup Mygaps
      (Variables|Default|SetMyGaps (Variables|/Game/Blueprints/TopPlatformSet.TopPlatformSet_C|GetGaps (Variables|Default|GetTopPlatformSet))))
    (:then_1
      (for _array_element _array
        ;[1 1 1] Set Initial Visibility
        (Rendering|SetVisibility _array_element false false)
        (Collision|SetCollisionEnabled _array_element "NoCollision"))
      ;[1 1 1] Setup Top Platform of New Set
      (for _array_element_2 _array
        (for _array_element_3 (Variables|Default|GetMyGaps)
          (if (and (Variables|Default|GetIsFirstMovingPlatform) (Variables|Default|GetFirstRun))
            (if (== _array_element_3 (+ (Math|Conversions|ToFloat(Integer) (Utilities|String|ToString(Object) _array_element_2)) 2.0))
              (Rendering|SetVisibility _array_element_2 true false :!label _label)
              (Collision|SetCollisionEnabled _array_element_2 "QueryAndPhysics")
              (Variables|Default|SetPlatformsVisible (+ (Variables|Default|GetPlatformsVisible) 1)))
            (elif (== _array_element_3 (+ (Math|Conversions|ToFloat(Integer) (Utilities|String|ToString(Object) _array_element_2)) 5.0))
              (goto _label)))))
      ;[1 1 1] Clear MyGaps
      (Utilities|Array|Clear (Variables|Default|GetMyGaps))
      ;[1 1 1] Setup Second Platform of New Set
      (for _array_element_4 _array
        (if (not (Rendering|IsVisible _array_element_4))
          (if (< (Variables|Default|GetPlatformsVisible) 5)
            (Rendering|SetVisibility _array_element_4 (> (Math|Random|RandomFloatinRange 0.0 1.0) 0.5) false)
            (if (Rendering|IsVisible _array_element_4)
              (Collision|SetCollisionEnabled _array_element_4 "QueryAndPhysics")
              (Variables|Default|SetPlatformsVisible (+ (Variables|Default|GetPlatformsVisible) 1))
              (else
                (Utilities|Array|Add (Variables|Default|GetMyGaps) (Math|Conversions|ToFloat(Integer) (Utilities|String|ToString(Object) _array_element_4)) :!label _label_2)))
            (else
              (goto _label_2))))))
    (:then_2
      ;[1 1 1] Rows 2-6
      (CallFunction|GeneratePlatforms (Utilities|Array|MakeArray (Variables|PlatformMeshes|Get2.1) (Variables|PlatformMeshes|Get2.2) (Variables|PlatformMeshes|Get2.3) (Variables|PlatformMeshes|Get2.4) (Variables|PlatformMeshes|Get2.5) (Variables|PlatformMeshes|Get2.6)))
      (CallFunction|GeneratePlatforms (Utilities|Array|MakeArray (Variables|PlatformMeshes|Get3.1) (Variables|PlatformMeshes|Get3.2) (Variables|PlatformMeshes|Get3.3) (Variables|PlatformMeshes|Get3.4) (Variables|PlatformMeshes|Get3.5) (Variables|PlatformMeshes|Get3.6)))
      (CallFunction|GeneratePlatforms (Utilities|Array|MakeArray (Variables|Default|Get4.1) (Variables|Default|Get4.2) (Variables|Default|Get4.3) (Variables|Default|Get4.4) (Variables|Default|Get4.5) (Variables|Default|Get4.6)))
      (CallFunction|GeneratePlatforms (Utilities|Array|MakeArray (Variables|Default|Get5.1) (Variables|Default|Get5.2) (Variables|Default|Get5.3) (Variables|Default|Get5.4) (Variables|Default|Get5.5) (Variables|Default|Get5.6)))
      (CallFunction|GeneratePlatforms (Utilities|Array|MakeArray (Variables|Default|Get6.1) (Variables|Default|Get6.2) (Variables|Default|Get6.3) (Variables|Default|Get6.4) (Variables|Default|Get6.5) (Variables|Default|Get6.6))))))

(event EventBeginPlay
  ;[1 1 1] Entry Point
  (Utilities|FlowControl|Sequence
    (:then_0
      ;[1 1 1] Get from Top Platform
      (bind _outactors (Actor|GetAllActorsOfClass "/Game/Blueprints/TopPlatformSet.TopPlatformSet_C"))
      (bind _astop_platform_set (Utilities|Casting|CastToTopPlatformSet (Utilities|Array|Get(acopy) _outactors)))
      (Variables|Default|SetTopPlatformSet _astop_platform_set))
    (:then_1
      ;[1 1 1] Setup Current Platform
      (bind _outactors_2 (Actor|GetAllActorsOfClass "UpperPlatformSet_C"))
      (for _array_element _outactors_2
        (if (not (Utilities|Enum|Equal(Enum) (Utilities|GetDisplayName _array_element) (Utilities|GetDisplayName self)))
          (bind _asupper_platform_set (Utilities|Casting|CastToUpperPlatformSet _array_element))
          (Variables|Default|SetOtherSwappingPlatform _asupper_platform_set))))
    (:then_2
      (Variables|Default|SetFirstRun true))))

(fn ConstructionScript)

(fn GeneratePlatforms
  (params (PlatformsArray :type Array%20of%20Static%20Mesh%20Component%20Object%20References))
  (Variables|Default|SetPlatformsVisible 0)
  ;[1 1 1] Setup Intial Settings
  (for _array_element PlatformsArray
    (Rendering|SetVisibility _array_element false false)
    (Collision|SetCollisionEnabled _array_element "NoCollision"))
  ;[1 1 1] Draw Platforms or Gaps
  (for _array_element_2 PlatformsArray
    (for _array_element_3 (Variables|Default|GetMyGaps)
      (if (== (+ _array_element_3 1.0) (Math|Conversions|ToFloat(Integer) (Utilities|String|ToString(Object) _array_element_2)))
        (Rendering|SetVisibility _array_element_2 true false)
        (Collision|SetCollisionEnabled _array_element_2 "QueryAndPhysics")
        (Variables|Default|SetPlatformsVisible (+ (Variables|Default|GetPlatformsVisible) 1)))))
  ;[1 1 1] Clear MyGaps
  (Utilities|Array|Clear (Variables|Default|GetMyGaps))
  ;[1 1 1] Setup Next Platform
  (for _array_element_4 PlatformsArray
    (if (not (Rendering|IsVisible _array_element_4))
      (if (< (Variables|Default|GetPlatformsVisible) 5)
        (Rendering|SetVisibility _array_element_4 (> (Math|Random|RandomFloatinRange 0.0 1.0) 0.5) false)
        (if (Rendering|IsVisible _array_element_4)
          (Collision|SetCollisionEnabled _array_element_4 "QueryAndPhysics")
          (Variables|Default|SetPlatformsVisible (+ (Variables|Default|GetPlatformsVisible) 1))
          (else
            (Utilities|Array|Add (Variables|Default|GetMyGaps) (Math|Conversions|ToFloat(Integer) (Utilities|String|ToString(Object) _array_element_4)) :!label _label)))
        (else
          (goto _label))))))