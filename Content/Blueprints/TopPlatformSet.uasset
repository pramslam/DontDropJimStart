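; TopPlatformSet lays out a randomized starting set of three platform rows on BeginPlay by toggling visibility and collision.
; Row one is fixed; row two randomly fills around one fixed platform, capped at five, recording hidden slots as Gaps.
; Component names convert to floats, so gap plus 1.0 forces the row-three platform above visible before random filling.
; Row-three gaps are stored for the next set, then CreateSelf runs on the first moving UpperPlatformSet.
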(event EventBeginPlay
  (bind _1_1 (Variables|PlatformMeshes|Get1.1))
  (bind _1_4 (Variables|PlatformMeshes|Get1.4))
  (bind _2_4 (Variables|PlatformMeshes|Get2.4))
  ;[1 1 1] Setup Starting Platforms
  (Rendering|SetVisibility _1_1 true false)
  (Collision|SetCollisionEnabled _1_1 "QueryAndPhysics")
  (Rendering|SetVisibility _1_4 false false)
  (Collision|SetCollisionEnabled _1_4 "NoCollision")
  (Rendering|SetVisibility _2_4 true false)
  (Collision|SetCollisionEnabled _2_4 "QueryAndPhysics")
  (Variables|Default|SetPlatformsVisible 1)
  (Rendering|SetVisibility (Variables|PlatformMeshes|Get2.1) false false)
  (Collision|SetCollisionEnabled (Variables|PlatformMeshes|Get2.6) "NoCollision")
  ;[1 1 1] Level 2 Platforms
  (for _array_element (Utilities|Array|MakeArray (Variables|PlatformMeshes|Get2.1) (Variables|PlatformMeshes|Get2.2) (Variables|PlatformMeshes|Get2.3) (Variables|PlatformMeshes|Get2.4) (Variables|PlatformMeshes|Get2.5) (Variables|PlatformMeshes|Get2.6))
    (if (not (Rendering|IsVisible _array_element))
      (if (< (Variables|Default|GetPlatformsVisible) 5)
        (Rendering|SetVisibility _array_element (> (Math|Random|RandomFloatinRange 0.0 1.0) 0.5) false)
        (if (Rendering|IsVisible _array_element)
          (Collision|SetCollisionEnabled _array_element "QueryAndPhysics")
          (Variables|Default|SetPlatformsVisible (+ (Variables|Default|GetPlatformsVisible) 1))
          (else
            (Utilities|Array|Add (Variables|Default|GetGaps) (Math|Conversions|ToFloat(Integer) (Utilities|String|ToString(Object) _array_element)) :!label _label)))
        (else
          (goto _label)))))
  ;[1 1 1] Level 3 Platforms
  (Variables|Default|SetPlatformsVisible 0)
  (for _array_element_2 (Utilities|Array|MakeArray (Variables|PlatformMeshes|Get3.1) (Variables|PlatformMeshes|Get3.2) (Variables|PlatformMeshes|Get3.3) (Variables|PlatformMeshes|Get3.4) (Variables|PlatformMeshes|Get3.5) (Variables|PlatformMeshes|Get3.6))
    (Rendering|SetVisibility _array_element_2 false false)
    (Collision|SetCollisionEnabled _array_element_2 "NoCollision")
    (for _array_element_3 (Variables|Default|GetGaps)
      (if (== (+ _array_element_3 1.0) (Math|Conversions|ToFloat(Integer) (Utilities|String|ToString(Object) _array_element_2)))
        (Rendering|SetVisibility _array_element_2 true false)
        (Collision|SetCollisionEnabled _array_element_2 "QueryAndPhysics")
        (Variables|Default|SetPlatformsVisible (+ (Variables|Default|GetPlatformsVisible) 1)))))
  ;[1 1 1] Clear Array
  (Utilities|Array|Clear (Variables|Default|GetGaps))
  ;[1 1 1] Setup Platforms for next Platform object
  (for _array_element_4 (Utilities|Array|MakeArray (Variables|PlatformMeshes|Get3.1) (Variables|PlatformMeshes|Get3.2) (Variables|PlatformMeshes|Get3.3) (Variables|PlatformMeshes|Get3.4) (Variables|PlatformMeshes|Get3.5) (Variables|PlatformMeshes|Get3.6))
    (if (not (Rendering|IsVisible _array_element_4))
      (if (< (Variables|Default|GetPlatformsVisible) 5)
        (Rendering|SetVisibility _array_element_4 (> (Math|Random|RandomFloatinRange 0.0 1.0) 0.5) false)
        (if (Rendering|IsVisible _array_element_4)
          (Collision|SetCollisionEnabled _array_element_4 "QueryAndPhysics")
          (Variables|Default|SetPlatformsVisible (+ (Variables|Default|GetPlatformsVisible) 1))
          (else
            (Utilities|Array|Add (Variables|Default|GetGaps) (Math|Conversions|ToFloat(Integer) (Utilities|String|ToString(Object) _array_element_4)) :!label _label_2)))
        (else
          (goto _label_2)))))
  (Utilities|FlowControl|Delay 0.2)
  (bind _outactors (Actor|GetAllActorsOfClass "/Game/Blueprints/UpperPlatformSet.UpperPlatformSet_C"))
  (bind _array_element_5 (Utilities|Array|ForEachLoopwithBreak _outactors :!label _label_3)
    (:LoopBody
      (bind _asupper_platform_set (Utilities|Casting|CastToUpperPlatformSet _array_element_5))
      (if (Variables|/Game/Blueprints/UpperPlatformSet.UpperPlatformSet_C|GetIsFirstMovingPlatform _asupper_platform_set)
        (Variables|Default|SetTopSwappingPlatform _asupper_platform_set)
        (goto _label_3 Break)))
    (:Completed
      (Default|CreateSelf (Variables|Default|GetTopSwappingPlatform)))))

(fn ConstructionScript)