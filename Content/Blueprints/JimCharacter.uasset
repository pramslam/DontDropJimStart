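; Player character Blueprint that runs automatically along the world Y axis, reversing direction when the actor is clicked.
; BeginPlay caches the JimGame game mode and starts an endless Delay loop that ramps walk speed up to a cap.
; A click FlipFlop rotates the actor, sets the direction flag read by Tick's movement input, and resets the Speed variable.
; The game mode's CanMovePlayer flag gates acceleration, turning and movement.
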(event EventBeginPlay
  ;[1 1 1] Set the Game Mode
  (bind _asjim_game (Utilities|Casting|CastToJimGame (Game|GetGameMode)))
  (Variables|Default|SetJimGameStore _asjim_game)
  ;[1 1 1] Set Initial Rotation
  (Transformation|SetActorRotation (Variables|Default|GetRightDirectionPawn))
  ;[1 1 1] Acceleration (Loops Infinitely)
  (if (<= (Variables|Default|GetSpeed) 375.0) :!label _label
    (if (Variables|/Game/Blueprints/JimGame.JimGame_C|GetCanMovePlayer (Variables|Default|GetJimGameStore))
      (Variables|Default|SetSpeed (+ (Variables|Default|GetSpeed) (Variables|Default|GetSpeedIncrease)))
      (Variables|/Script/Engine.CharacterMovementComponent|SetMaxWalkSpeed (Variables|Character|GetCharacterMovement) (Variables|Default|GetSpeed))
      (Utilities|FlowControl|Delay (Variables|Default|GetRateIncrease))
      (goto _label)
      (else
        _)))
  (Utilities|FlowControl|Delay 0.1)
  (goto _label))

(event MouseInput|EventActorOnClicked
  ;[1 1 1] Set Actor Rotation
  (if (Variables|/Game/Blueprints/JimGame.JimGame_C|GetCanMovePlayer (Variables|Default|GetJimGameStore))
    (Utilities|FlowControl|FlipFlop
      (:A
        (Variables|Default|SetFlipDirection false)
        (Transformation|AddActorLocalRotation (Variables|Default|GetRightDirectionPawn) false false)
        (Variables|Default|SetSpeed 1.6e+02))
      (:B
        (Variables|Default|SetFlipDirection true)
        (Transformation|AddActorLocalRotation (Variables|Default|GetLeftDirectionPawn) false false)
        (Variables|Default|SetSpeed 1.6e+02)))))

(event EventTick
  (params (DeltaSeconds :type Float%20%28single-precision%29))
  (bind _returnvalue (Transformation|GetActorLocation))
  ;[1 1 1] Set Movement
  (if (Variables|/Game/Blueprints/JimGame.JimGame_C|GetCanMovePlayer (Variables|Default|GetJimGameStore))
    (if (Variables|Default|GetFlipDirection)
      (Pawn|Input|AddMovementInput (Math|Transform|TransformDirection (Math|Conversions|ToTransform(Vector) _returnvalue) "0.000000,-1.000000, 0") 1.0 false)
      (else
        (Pawn|Input|AddMovementInput (Math|Transform|TransformDirection (Math|Conversions|ToTransform(Vector) _returnvalue) "0,1.000000, 0") 1.0 false)))))

(fn ConstructionScript)